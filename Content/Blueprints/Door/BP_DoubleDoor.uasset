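; BP_DoubleDoor is an automatic sliding double door that opens when the player character enters its box trigger and closes when they leave.
; Overlap begin and end events filter for CMP407_ReverberationCharacter and play an audio component for each door on both opening and closing.
; Two float timelines each drive one door mesh's relative X location, playing forward to open and reversing to close.
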(event OnComponentBeginOverlap(Box)
  (params (OverlappedComponent :type Primitive%20Component%20Object%20Reference) (OtherActor :type Actor%20Object%20Reference) (OtherComp :type Primitive%20Component%20Object%20Reference) (OtherBodyIndex :type Integer) (bFromSweep :type Boolean) (SweepResult :type Hit%20Result%20Structure%20%28by%20ref%29))
  ;[1 1 1] If player overlaps with the doors box collider, play the door open sound on BOTH doors.
  (Utilities|Casting|CastToCMP407_ReverberationCharacter OtherActor)
  (Audio|Components|Audio|Play (Variables|Default|GetDoorAudioComponent) 0.0)
  (Audio|Components|Audio|Play (Variables|Default|GetDoorAudioComponent1) 0.0)
  (Utilities|FlowControl|Sequence
    (:then_0
      ;[1 1 1] Play timeline on a float curve on BOTH doors, adjusting the door values to make them move away over time period
      (bind _doortrack (Timeline|Door%20Open%20Timeline Play)
        (:Update
          (Transformation|SetRelativeLocation (Variables|Default|GetDoorMesh) (Math|Vector|MakeVector _doortrack 0.0 0.0) false false))))
    (:then_1
      (bind _doortrack_2 (Timeline|Other%20Door%20Open%20Timeline Play)
        (:Update
          (Transformation|SetRelativeLocation (Variables|Default|GetDoorMesh1) (Math|Vector|MakeVector _doortrack_2 0.0 0.0) false false))))))

(event OnComponentEndOverlap(Box)
  (params (OverlappedComponent :type Primitive%20Component%20Object%20Reference) (OtherActor :type Actor%20Object%20Reference) (OtherComp :type Primitive%20Component%20Object%20Reference) (OtherBodyIndex :type Integer))
  ;[1 1 1] If player overlaps with the doors box collider, play the door open sound on BOTH doors.
  (Utilities|Casting|CastToCMP407_ReverberationCharacter OtherActor)
  (Audio|Components|Audio|Play (Variables|Default|GetDoorAudioComponent) 0.0)
  (Audio|Components|Audio|Play (Variables|Default|GetDoorAudioComponent1) 0.0)
  (Utilities|FlowControl|Sequence
    (:then_0
      ;[1 1 1] Play timeline on a float curve on BOTH doors, adjusting the door values to make them move away over time period
      (bind _doortrack (Timeline|Door%20Open%20Timeline Reverse)
        (:Update
          (Transformation|SetRelativeLocation (Variables|Default|GetDoorMesh) (Math|Vector|MakeVector _doortrack 0.0 0.0) false false))))
    (:then_1
      (bind _doortrack_2 (Timeline|Other%20Door%20Open%20Timeline Reverse)
        (:Update
          (Transformation|SetRelativeLocation (Variables|Default|GetDoorMesh1) (Math|Vector|MakeVector _doortrack_2 0.0 0.0) false false))))))

(event EventBeginPlay)

(event Collision|EventActorBeginOverlap
  (params (OtherActor :type Actor%20Object%20Reference)))

(event EventTick
  (params (DeltaSeconds :type Float%20%28single-precision%29)))

(fn ConstructionScript)